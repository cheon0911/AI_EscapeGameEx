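; BP_Door is a door that swings open when its box trigger is overlapped, provided no second-floor coins remain uncollected.
; On overlap, CoinCheck counts BaseItem actors flagged IsOn2F; at zero, a timeline lerps the door's yaw open, otherwise it prints a collect-coin message.
; Ending the overlap always plays a second timeline from the start to swing the door shut, even if it never opened.
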(event OnComponentBeginOverlap(Box)
  (params (OverlappedComponent :type Primitive%20Component%20Object%20Reference) (OtherActor :type Actor%20Object%20Reference) (OtherComp :type Primitive%20Component%20Object%20Reference) (OtherBodyIndex :type Integer) (bFromSweep :type Boolean) (SweepResult :type Hit%20Result%20Structure%20%28by%20ref%29))
  (bind _door (Variables|Default|GetDoor))
  (bind _relativerotation (Variables|/Script/Engine.SceneComponent|GetRelativeRotation _door))
  (CallFunction|CoinCheck)
  (if (>= 0 (Variables|Default|Get2FCoin))
    (bind _newtrack_0 (Timeline|DoorOpen PlayFromStart)
      (:Update
        (Transformation|SetRelativeRotation _door (Math|Rotator|MakeRotator (.roll _relativerotation) (.pitch _relativerotation) (Math|Float|Lerp 0.0 9e+01 _newtrack_0)) false false)))
    (else
      (Development|PrintString "Should collect coin"))))

(event OnComponentEndOverlap(Box)
  (params (OverlappedComponent :type Primitive%20Component%20Object%20Reference) (OtherActor :type Actor%20Object%20Reference) (OtherComp :type Primitive%20Component%20Object%20Reference) (OtherBodyIndex :type Integer))
  (bind _door (Variables|Default|GetDoor))
  (bind _relativerotation (Variables|/Script/Engine.SceneComponent|GetRelativeRotation _door))
  (bind _newtrack_0 (Timeline|Timeline PlayFromStart)
    (:Update
      (Transformation|SetRelativeRotation _door (Math|Rotator|MakeRotator (.roll _relativerotation) (.pitch _relativerotation) (Math|Float|Lerp 9e+01 0.0 _newtrack_0)) false false))))

(event Custom|CoinCheck
  (bind _outactors (Actor|GetAllActorsOfClass "/Script/AI_EscapeGameEx.BaseItem"))
  (Variables|Default|Set2FCoin 0)
  (for _array_element _outactors
    (if (Variables|/Script/AI_EscapeGameEx.BaseItem|GetbIsOn2F _array_element)
      (Math|Integer|IncrementInt (Variables|Default|Get2FCoin))))
  (Development|PrintString (Utilities|String|ToString(Integer) (Variables|Default|Get2FCoin))))

(event EventBeginPlay)

(event Collision|EventActorBeginOverlap
  (params (OtherActor :type Actor%20Object%20Reference)))

(event EventTick
  (params (DeltaSeconds :type Float%20%28single-precision%29)))

(fn ConstructionScript)